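; AI controller for Enemy_base pawns that runs the AiBT behavior tree and feeds its blackboard.
; On BeginPlay it copies the pawn's patrol path loop and wait settings and sets the starting direction.
; Perception updates pass stimuli to Senses, which tells senses apart by array index: the first flags CanSeePlayer, while the next two flag investigation and store the stimulus location.
; Only successful stimuli write keys; nothing here clears them.
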(event `self.ReceiveBeginPlay`
  (bind _returnvalue (`AIBlueprintHelperLibrary.GetBlackboard` null))
  (`self.RunBehaviorTree` "/Game/Ai/Ai-BT.Ai-BT")
  (bind _asenemy_base (cast `/Game/Ai/Enemy_base` (`self.K2_GetPawn`)))
  (bind _output_get (set `self.MyPawn` _asenemy_base))
  (`BlackboardComponent.SetValueAsBool` (`AIBlueprintHelperLibrary.GetBlackboard` null) "Pathloop" (`/Game/Ai/Patrolpath.IsLooping` (`/Game/Ai/Enemy_base.PatrolPath` _output_get)))
  (`BlackboardComponent.SetValueAsInt` _returnvalue "Direction" 1)
  (`BlackboardComponent.SetValueAsFloat` _returnvalue "WaitTime" (`/Game/Ai/Patrolpath.WaitTime` (`/Game/Ai/Enemy_base.PatrolPath` (`self.MyPawn`)))))

(event `self.AIPerception.OnPerceptionUpdated`
  (params (UpdatedActors :type "Array of Actor Object Reference (by ref)"))
  (for _array_element UpdatedActors
    (bind _info (`AIPerceptionComponent.GetActorsPerception` (`self.AIPerception`) _array_element))
    (`self.Senses` (`.LastSensedStimuli` (break `ActorPerceptionBlueprintInfo` _info)))))

(fn `Senses`
  (params (Array :type "Array of AIStimulus Structure"))
  (bind _returnvalue (`AIBlueprintHelperLibrary.GetBlackboard` null))
  (bind (_local_sense_age _local_sense_expirationage _local_sense_strength _local_sense_stimuluslocation _local_sense_receiverlocation _local_sense_tag _local_sense_bsuccessfullysensed) (break `AIStimulus` (`self.Local Sense`)))
  (bind (_local_sense_age_2 _local_sense_expirationage_2 _local_sense_strength_2 _local_sense_stimuluslocation_2 _local_sense_receiverlocation_2 _local_sense_tag_2 _local_sense_bsuccessfullysensed_2) (break `AIStimulus` (`self.Local Sense`)))
  (for (_array_element _array_index) Array
    (set `self.Local Sense` _array_element)
    (switch `int` _array_index
      (:`0`
        (if _local_sense_bsuccessfullysensed
          (`BlackboardComponent.SetValueAsBool` (`AIBlueprintHelperLibrary.GetBlackboard` null) "CanSeePlayer" _local_sense_bsuccessfullysensed)))
      (:`1`
        (if _local_sense_bsuccessfullysensed
          (`BlackboardComponent.SetValueAsBool` _returnvalue "IsInvestigating" _local_sense_bsuccessfullysensed_2 :!label _label)
          (`BlackboardComponent.SetValueAsVector` _returnvalue "Target_location" _local_sense_stimuluslocation_2)))
      (:`2`
        (if _local_sense_bsuccessfullysensed
          (goto _label))))))

(fn `UserConstructionScript`)