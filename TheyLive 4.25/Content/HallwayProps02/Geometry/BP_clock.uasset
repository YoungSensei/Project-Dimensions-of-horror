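; A wall or hallway clock prop that displays a set time and can animate its second hand.
; The construction script converts Hour and Minute into roll rotations on two sets of hand pivots, with opposite signs and separate offsets for each set.
; On BeginPlay, if Animate is on, a timeline's Time track drives the roll of the single second-hand pivot; hour and minute hands stay static.
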(event `self.ReceiveBeginPlay`
  (if (`self.Animate`)
    (bind (_direction _time) (`Timeline|Timeline_0`)
      (:`Update`
        (`SceneComponent.K2_SetRelativeRotation` (`self.SecondHandPivot`) (`KismetMathLibrary.MakeRotator` _time) false false)))))

(fn `UserConstructionScript`
  (`SceneComponent.K2_SetRelativeRotation` (`self.HourHandPivot`) (`KismetMathLibrary.MakeRotator` (`KismetMathLibrary.Conv_IntToDouble` (+ (* (`self.Hour`) -30) 2))) false false)
  (`SceneComponent.K2_SetRelativeRotation` (`self.MinuteHandPivot`) (`KismetMathLibrary.MakeRotator` (`KismetMathLibrary.Conv_IntToDouble` (+ (* (`self.Minute`) -6) 2))) false false)
  (`SceneComponent.K2_SetRelativeRotation` (`self.HourHandPivot02`) (`KismetMathLibrary.MakeRotator` (`KismetMathLibrary.Conv_IntToDouble` (+ (* (`self.Hour`) 30) 87))) false false)
  (`SceneComponent.K2_SetRelativeRotation` (`self.MinuteHandPivot02`) (`KismetMathLibrary.MakeRotator` (`KismetMathLibrary.Conv_IntToDouble` (+ (* (`self.Minute`) 6) 199))) false false))