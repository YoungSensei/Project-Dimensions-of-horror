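; An interactable door Blueprint that swings open and closed when the player presses Interact.
; Overlapping its Box component enables input from player controller 0, and ending the overlap disables it, with no check on which actor overlaps.
; An IsClosed flag toggles the DoorOpenClose timeline between Play and Reverse.
; The timeline's Door track sets the mesh's absolute world yaw, so the door's placed rotation is overridden.
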(event `self.Box.OnComponentBeginOverlap`
  (params (OverlappedComponent :type "PrimitiveComponent Object Reference") (OtherActor :type "Actor Object Reference") (OtherComp :type "PrimitiveComponent Object Reference") (OtherBodyIndex :type Integer) (bFromSweep :type Boolean) (SweepResult :type "HitResult Structure (by ref)"))
  (`self.EnableInput` (`GameplayStatics.GetPlayerController` 0)))

(event `self.Box.OnComponentEndOverlap`
  (params (OverlappedComponent :type "PrimitiveComponent Object Reference") (OtherActor :type "Actor Object Reference") (OtherComp :type "PrimitiveComponent Object Reference") (OtherBodyIndex :type Integer))
  (`self.DisableInput` (`GameplayStatics.GetPlayerController` 0)))

(event `InputAction|Interact`
  (params (Key :type "Key Structure"))
  (:`Pressed`
    (if (`self.Is Closed`)
      (set `self.Is Closed` false)
      (bind (_direction _door) (`Timeline|Door Open/Close` :!label _label)
        (:`Update`
          (`SceneComponent.K2_SetWorldRotation` (`self.StaticMesh1`) (`KismetMathLibrary.MakeRotator` 0.0 0.0 _door) false false)))
      (else
        (set `self.Is Closed` true)
        (goto _label :!via `Reverse`)))))

(fn `UserConstructionScript`)