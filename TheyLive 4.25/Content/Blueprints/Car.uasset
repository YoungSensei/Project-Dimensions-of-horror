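; Car is an interactable that takes the player to the Parkour level if they hold the required key.
; Its Box overlap casts to ThirdPersonCharacter and checks Keys at KeyValue, showing an AxePickup widget and enabling input, or a NeedKey widget and a debug print.
; While input is enabled, Interact shows a LoadingScreen and opens the level.
; Leaving the box disables input but leaves the prompt widgets on screen.
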(event `self.Box.OnComponentBeginOverlap`
  (params (OverlappedComponent :type "PrimitiveComponent Object Reference") (OtherActor :type "Actor Object Reference") (OtherComp :type "PrimitiveComponent Object Reference") (OtherBodyIndex :type Integer) (bFromSweep :type Boolean) (SweepResult :type "HitResult Structure (by ref)"))
  (bind _asthird_person_character (cast `/Game/ThirdPersonBP/Blueprints/ThirdPersonCharacter` OtherActor))
  (if (`|GetArrayItem` (`/Game/ThirdPersonBP/Blueprints/ThirdPersonCharacter.keys` _asthird_person_character) (`self.key_value`))
    (bind _returnvalue (`|CreateWidget` "/Game/Blueprints/Widgets/AxePickup.AxePickup_C"))
    (`UserWidget.AddToViewport` _returnvalue 0)
    (`self.EnableInput` (`GameplayStatics.GetPlayerController` 0))
    (else
      (bind _returnvalue_2 (`|CreateWidget` "/Game/Blueprints/Widgets/NeedKey.NeedKey_C"))
      (`UserWidget.AddToViewport` _returnvalue_2 0)
      (`KismetSystemLibrary.PrintString` "Hello"))))

(event `self.Box.OnComponentEndOverlap`
  (params (OverlappedComponent :type "PrimitiveComponent Object Reference") (OtherActor :type "Actor Object Reference") (OtherComp :type "PrimitiveComponent Object Reference") (OtherBodyIndex :type Integer))
  (`self.DisableInput` (`GameplayStatics.GetPlayerController` 0)))

(event `InputAction|Interact`
  (params (Key :type "Key Structure"))
  (:`Pressed`
    (bind _returnvalue (`|CreateWidget` "/Game/Blueprints/Widgets/LoadingScreen.LoadingScreen_C"))
    (`UserWidget.AddToViewport` _returnvalue 0)
    (`GameplayStatics.OpenLevel` "Parkour")))

(fn `UserConstructionScript`)