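; AI controller for the ranged enemy that runs its behavior tree when it possesses a RangedAI pawn.
; Perception updates on the player character write the player reference and visibility to the Blackboard.
; When sight is lost, it also stores the player's current location and flags them as recently sighted.
; Walk, Run and Attack events forward to the possessed enemy.
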(event `self.AIPerception.OnTargetPerceptionUpdated`
  (params (Actor :type "Actor Object Reference") (Stimulus :type "AIStimulus Structure"))
  (bind (_age _expirationage _strength _stimuluslocation _receiverlocation _tag _bsuccessfullysensed) (break `AIStimulus` Stimulus))
  (bind _returnvalue (`AIBlueprintHelperLibrary.GetBlackboard` null))
  (bind _returnvalue_2 (`GameplayStatics.GetPlayerCharacter` 0))
  (cast `/Game/ThirdPersonBP/Blueprints/ThirdPersonCharacter` Actor)
  (`BlackboardComponent.SetValueAsObject` _returnvalue "PlayerReference" _returnvalue_2)
  (`BlackboardComponent.SetValueAsBool` _returnvalue "CanSeePlayer" _bsuccessfullysensed)
  (if (not _bsuccessfullysensed)
    (`BlackboardComponent.SetValueAsVector` _returnvalue "PlayerLocation" (`self.K2_GetActorLocation` _returnvalue_2))
    (`BlackboardComponent.SetValueAsBool` _returnvalue "RecentlySighted" true)))

(event `Walk`
  (`/Game/Blueprints/RangedAI/RangedAI.Walk` (`self.RangedEnemy`)))

(event `Run`
  (`/Game/Blueprints/RangedAI/RangedAI.Run` (`self.RangedEnemy`)))

(event `self.ReceivePossess`
  (params (PossessedPawn :type "Pawn Object Reference"))
  (bind _asranged_ai (cast `/Game/Blueprints/RangedAI/RangedAI` PossessedPawn))
  (set `self.RangedEnemy` _asranged_ai)
  (`self.RunBehaviorTree` "/Game/Blueprints/RangedAI/RangedAI-BT.RangedAI-BT"))

(event `Attack`
  (`/Game/Blueprints/RangedAI/RangedAI.Attack` (`self.RangedEnemy`)))

(fn `UserConstructionScript`)