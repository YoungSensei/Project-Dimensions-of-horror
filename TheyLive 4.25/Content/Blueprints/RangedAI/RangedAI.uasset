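; RangedAI is a shotgun-wielding AI character Blueprint with events for walking, running and attacking.
; Walk and Run switch the CharacterMovement max speed between slow and fast.
; Attack plays a hip-fire animation and runs a debug-drawn visibility line trace from above the actor's location along control rotation.
; The ThirdPersonCharacter hit check and the return to Animation Blueprint mode are unconnected, so hits have no effect.
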(event `Walk`
  (set `CharacterMovementComponent.MaxWalkSpeed` 150.0 (`self.CharacterMovement`)))

(event `Run`
  (set `CharacterMovementComponent.MaxWalkSpeed` 600.0 (`self.CharacterMovement`)))

(event `Attack`
  (bind _returnvalue (`KismetMathLibrary.MakeVector` (.x (`self.K2_GetActorLocation`)) (.y (`self.K2_GetActorLocation`)) (+ (.z (`self.K2_GetActorLocation`)) 60.0)))
  (`SkeletalMeshComponent.PlayAnimation` (`self.Mesh`) "/Game/AnimStarterPack/Fire_Shotgun_Hip.Fire_Shotgun_Hip" false)
  (bind _outhit (`KismetSystemLibrary.LineTraceSingle` :`Start` _returnvalue :`End` (+ _returnvalue (* (`KismetMathLibrary.Conv_RotatorToVector` (`self.GetControlRotation`)) 2500.0)) :`TraceChannel` "TraceTypeQuery1" :`DrawDebugType` "ForDuration")))

(fn `UserConstructionScript`)