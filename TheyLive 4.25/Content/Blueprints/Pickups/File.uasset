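; Pickup actor that the player collects into their inventory by pressing Interact while it accepts input.
; Box overlap enables input from player controller 0 for any overlapping actor, and end overlap disables it.
; Interact casts the overlap's OtherActor to ThirdPersonCharacter, inserts the item's Data at the front of its Inventory, shows a KeyPopup widget and destroys the pickup.
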(event `self.Box.OnComponentBeginOverlap`
  (params (OverlappedComponent :type "PrimitiveComponent Object Reference") (OtherActor :type "Actor Object Reference") (OtherComp :type "PrimitiveComponent Object Reference") (OtherBodyIndex :type Integer) (bFromSweep :type Boolean) (SweepResult :type "HitResult Structure (by ref)"))
  (`self.EnableInput` (`GameplayStatics.GetPlayerController` 0)))

(event `self.Box.OnComponentEndOverlap`
  (params (OverlappedComponent :type "PrimitiveComponent Object Reference") (OtherActor :type "Actor Object Reference") (OtherComp :type "PrimitiveComponent Object Reference") (OtherBodyIndex :type Integer))
  (`self.DisableInput` (`GameplayStatics.GetPlayerController` 0)))

(event `InputAction|Interact`
  (params (Key :type "Key Structure"))
  (:`Pressed`
    (bind _asthird_person_character (cast `/Game/ThirdPersonBP/Blueprints/ThirdPersonCharacter` (stale `self.Box.OnComponentBeginOverlap` OtherActor)))
    (`KismetArrayLibrary.Array_Insert` (`/Game/ThirdPersonBP/Blueprints/ThirdPersonCharacter.Inventory` _asthird_person_character) (`self.Data`))
    (bind _returnvalue (`|CreateWidget` "/Game/Blueprints/Widgets/KeyPopup.KeyPopup_C"))
    (`UserWidget.AddToViewport` _returnvalue 0)
    (`self.K2_DestroyActor`)))

(fn `UserConstructionScript`)