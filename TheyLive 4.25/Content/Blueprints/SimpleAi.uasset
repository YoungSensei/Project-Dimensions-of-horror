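; Simple enemy AI pawn that wanders, chases the player and takes projectile damage.
; A delayed Tick loop picks random nearby reachable points while no player is seen; PawnSensing starts a chase, cleared when the move ends.
; Projectile overlaps show a hit marker and reduce Health, spawning an impact effect and pursuing the player.
; At zero Health it spawns Ammo at the mesh's Drop socket and destroys itself.
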(event `self.ReceiveActorBeginOverlap`
  (params (OtherActor :type "Actor Object Reference"))
  (bind _asprojectile_base (cast `/Game/Blueprints/Projectile_Base` OtherActor))
  (bind _returnvalue (`|CreateWidget` "/Game/Blueprints/Widgets/HitMarker.HitMarker_C"))
  (`UserWidget.AddToViewport` _returnvalue 0)
  (bind _output_get (set `self.Health` (- (`self.Health`) 0.1)))
  (if (<= _output_get 0.0)
    (`|SpawnActorFromClass` "/Game/Blueprints/Pickups/Ammo.Ammo_C" (`SceneComponent.GetSocketTransform` (`self.Mesh`) "Drop" "RTS_World") "Undefined" "OverrideRootScale" null null)
    (`self.K2_DestroyActor`)
    (else
      (`GameplayStatics.SpawnEmitterAtLocation` "/Game/InfinityBladeEffects/Effects/FX_Mobile/ICE/combat/P_Impact_Shield.P_Impact_Shield" (`self.K2_GetActorLocation` _asprojectile_base))
      (bind _asthird_person_character (cast `/Game/ThirdPersonBP/Blueprints/ThirdPersonCharacter` (`GameplayStatics.GetPlayerCharacter` 0)))
      (`|AIMoveTo` self (0.0 0.0 0.0) _asthird_person_character))))

(event `self.PawnSensing.OnSeePawn`
  (params (Pawn :type "Pawn Object Reference"))
  (bind _asthird_person_character (cast `/Game/ThirdPersonBP/Blueprints/ThirdPersonCharacter` Pawn))
  (set `self.CanSee` true)
  (`|AIMoveTo` self (0.0 0.0 0.0) _asthird_person_character
    (:`OnSuccess`
      _)
    (:`OnFail`
      _))
  (set `self.CanSee` false))

(event `self.ReceiveTick`
  (params (DeltaSeconds :type "Float (single-precision)"))
  (`KismetSystemLibrary.Delay` 3.0)
  (if (not (`self.CanSee`))
    (`|AIMoveTo` self (`NavigationSystemV1.K2_GetRandomReachablePointInRadius` (`self.K2_GetActorLocation`) 250.0 null null) null)))

(fn `UserConstructionScript`)