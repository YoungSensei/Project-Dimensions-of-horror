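; Possessable locker that the player can hide in and exit again.
; On BeginPlay it caches the ThirdPersonCharacter and writes itself into that character's Locker variable.
; Box overlaps with the character open and close a gate, which both the Interact input and the Enter event feed.
; Each pass through the gate swaps player controller possession between character and locker, flips IsHiding and toggles the character mesh's visibility.
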(event `self.ReceiveBeginPlay`
  (bind _asthird_person_character (cast `/Game/ThirdPersonBP/Blueprints/ThirdPersonCharacter` (`GameplayStatics.GetPlayerCharacter` 0)))
  (set `self.Player` _asthird_person_character)
  (set `/Game/ThirdPersonBP/Blueprints/ThirdPersonCharacter.Locker` self _asthird_person_character))

(event `Enter`
  (bind _mesh (`Character.Mesh` (`self.Player`)))
  (`/Engine/EditorBlueprintResources/StandardMacros.Gate` true :!label _label
    (:`Exit`
      (if (`self.IsHiding`)
        (`Controller.Possess` (`GameplayStatics.GetPlayerController` 0) (`self.Player`))
        (set `self.IsHiding` false)
        (`SceneComponent.ToggleVisibility` _mesh false)
        (else
          (`Controller.Possess` (`GameplayStatics.GetPlayerController` 0) self)
          (set `self.IsHiding` true)
          (`SceneComponent.ToggleVisibility` _mesh false))))))

(event `InputAction|Interact`
  (params (Key :type "Key Structure"))
  (:`Pressed`
    (goto _label)))

(event `self.Box.OnComponentBeginOverlap`
  (params (OverlappedComponent :type "PrimitiveComponent Object Reference") (OtherActor :type "Actor Object Reference") (OtherComp :type "PrimitiveComponent Object Reference") (OtherBodyIndex :type Integer) (bFromSweep :type Boolean) (SweepResult :type "HitResult Structure (by ref)"))
  (cast `/Game/ThirdPersonBP/Blueprints/ThirdPersonCharacter` OtherActor)
  (goto _label :!via `Open`))

(event `self.Box.OnComponentEndOverlap`
  (params (OverlappedComponent :type "PrimitiveComponent Object Reference") (OtherActor :type "Actor Object Reference") (OtherComp :type "PrimitiveComponent Object Reference") (OtherBodyIndex :type Integer))
  (cast `/Game/ThirdPersonBP/Blueprints/ThirdPersonCharacter` OtherActor)
  (goto _label :!via `Close`))

(fn `UserConstructionScript`)