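; Game instance that handles saving, loading and clearing player progress in a single save slot.
; On Init it loads the existing My_Save object or creates a new one.
; Saving caches the ThirdPersonCharacter and writes its level name, location and inventory to the slot.
; Loading calls OpenLevel, then immediately applies location and inventory to that cached reference, which only SavePlayerData sets.
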(event `self.ReceiveInit`
  (bind _returnvalue (`GameplayStatics.DoesSaveGameExist` (`self.SaveSlot`)))
  (if _returnvalue
    (bind _returnvalue_2 (`GameplayStatics.LoadGameFromSlot` (`self.SaveSlot`)))
    (bind _asmy_save (cast `/Game/Blueprints/Save_System/My_Save` _returnvalue_2))
    (set `self.Save Game Data` _asmy_save)
    (else
      (bind _returnvalue_3 (`GameplayStatics.CreateSaveGameObject` "/Game/Blueprints/Save_System/My_Save.My_Save_C"))
      (set `self.Save Game Data` _returnvalue_3))))

(fn `Clear Save data`
  (`GameplayStatics.DeleteGameInSlot` (`self.SaveSlot`)))

(fn `Load Data`
  (bind _player_ref (`self.Player Ref`))
  (bind (_data_levelname _data_location _data_inven) (break `/Game/Blueprints/Save_System/PlayerData` (`/Game/Blueprints/Save_System/My_Save.Data` (`self.Save Game Data`))))
  (`GameplayStatics.OpenLevel` _data_levelname)
  (`Actor.K2_SetActorLocation` _player_ref _data_location false false)
  (set `/Game/ThirdPersonBP/Blueprints/ThirdPersonCharacter.Inventory` _data_inven _player_ref))

(fn `Save player Data`
  (bind _save_game_data (`self.Save Game Data`))
  (bind _player_ref (`self.Player Ref`))
  (bind _asthird_person_character (cast `/Game/ThirdPersonBP/Blueprints/ThirdPersonCharacter` (`GameplayStatics.GetPlayerCharacter` 0)))
  (set `self.Player Ref` _asthird_person_character)
  (bind _returnvalue (`GameplayStatics.GetCurrentLevelName` true))
  (set `/Game/Blueprints/Save_System/My_Save.Data` (make `/Game/Blueprints/Save_System/PlayerData` (`KismetStringLibrary.Conv_StringToName` _returnvalue) (`Actor.K2_GetActorLocation` _player_ref) (`/Game/ThirdPersonBP/Blueprints/ThirdPersonCharacter.Inventory` _player_ref)) _save_game_data)
  (`GameplayStatics.SaveGameToSlot` _save_game_data (`self.SaveSlot`)))